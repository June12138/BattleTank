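; Player-controllable tank pawn Blueprint that wires its barrel, turret, tracks and movement component together at BeginPlay.
; Aim inputs yaw an azimuth gimbal and pitch the spring arm to orbit the camera, and the Fire action calls Fire.
; Movement accepts either direct per-track throttle or forward/right intent axes routed through TankMovementComponent, which is initialised with both tracks.
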(event `self.ReceiveBeginPlay`
  (`self.SetBarrelReference` (`self.TankBarrel`))
  (`self.SetTurrentReference` (`self.Turrent`))
  (`TankMovementComponent.Init` (`self.TankMovementComponent`) (`self.LeftTrack`) (`self.RightTrack`)))

(event `InputAxis|AimAzimath`
  (params (AxisValue :type "Float (single-precision)"))
  ;[1 1 1] Camera setup
  (`SceneComponent.K2_AddLocalRotation` (`self.Azimuth Gible`) (`KismetMathLibrary.MakeRotator` 0.0 0.0 AxisValue) false false))

(event `InputAxis|AimElevation`
  (params (AxisValue :type "Float (single-precision)"))
  ;[1 1 1] Camera setup
  (`SceneComponent.K2_AddLocalRotation` (`self.SpringArm`) (`KismetMathLibrary.MakeRotator` 0.0 AxisValue) false false))

(event `InputAction|Fire`
  (params (Key :type "Key Structure"))
  (:`Pressed`
    (`self.Fire`)))

(event `InputAxis|LeftThrottle`
  (params (AxisValue :type "Float (single-precision)"))
  (`Track.SetThrottle` (`self.LeftTrack`) AxisValue))

(event `InputAxis|IntendMoveforward`
  (params (AxisValue :type "Float (single-precision)"))
  (`TankMovementComponent.IntendMoveForward` (`self.TankMovementComponent`) AxisValue))

(event `InputAxis|RightThrottle`
  (params (AxisValue :type "Float (single-precision)"))
  (`Track.SetThrottle` (`self.RightTrack`) AxisValue))

(event `InputAxis|IntendMoveRight`
  (params (AxisValue :type "Float (single-precision)"))
  (`TankMovementComponent.IntendMoveRight` (`self.TankMovementComponent`) AxisValue))

(fn `UserConstructionScript`)